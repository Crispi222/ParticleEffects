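; BP_Activator is an actor that switches a Target's particle effect on and off.
; Overlap begin and end with a BP_Character set or clear its own Overlapped flag and the character's IsTriggering flag.
; A separate Trigger event, with no caller in this Blueprint, toggles the Target's IsActive state and activates or deactivates its ParticleSystem to match.
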(event `self.ReceiveActorBeginOverlap`
  (params (OtherActor :type "Actor Object Reference"))
  (bind _asbp_character (cast `/Game/MyWork/Blueprints/BP_Character` OtherActor))
  (set `self.Overlapped` true)
  (set `/Game/MyWork/Blueprints/BP_Character.IsTriggering` true _asbp_character))

(event `self.ReceiveActorEndOverlap`
  (params (OtherActor :type "Actor Object Reference"))
  (bind _asbp_character (cast `/Game/MyWork/Blueprints/BP_Character` OtherActor))
  (set `self.Overlapped` false)
  (set `/Game/MyWork/Blueprints/BP_Character.IsTriggering` false _asbp_character))

(event `Trigger`
  (bind _target (`self.Target`))
  (bind _particlesystem (`/Game/MyWork/Blueprints/BP_Particle.ParticleSystem` _target))
  (if (`/Game/MyWork/Blueprints/BP_Particle.IsActive` _target)
    (set `/Game/MyWork/Blueprints/BP_Particle.IsActive` false (`self.Target`))
    (`ActorComponent.Deactivate` _particlesystem)
    (else
      (set `/Game/MyWork/Blueprints/BP_Particle.IsActive` true (`self.Target`))
      (`ActorComponent.Activate` _particlesystem false))))

(fn `UserConstructionScript`)